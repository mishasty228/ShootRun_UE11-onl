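; Default game mode that keeps a pool of weapon instances and switches the sound map's audio on and off.
; BeginPlay caches the level's attach actor and sound map actor.
; AddToPool stores a weapon without a validity check and snaps it to the attach actor; GetFromPool removes and returns one matching the requested class.
; ChangeCanMainSound activates or deactivates the sound map's audio component.
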(event `self.ReceiveBeginPlay`
  (bind _returnvalue (`GameplayStatics.GetActorOfClass` "/Game/Core/Blueprints/Character/Enemy/BP_AttachActor.BP_AttachActor_C"))
  (set `self.BP_AttachActor` _returnvalue)
  (bind _returnvalue_2 (`GameplayStatics.GetActorOfClass` "/Game/Sound/BP_SoundMap.BP_SoundMap_C"))
  (set `self.BP_SoundMap` _returnvalue_2))

(fn `AddToPool`
  (params (NewItem :type "/Game/Core/Blueprints/Weapons/BP_BaseWeapon Object Reference (by ref)"))
  (`KismetArrayLibrary.Array_Add` (`self.WeaponsClasses`) NewItem)
  (`self.K2_AttachToActor` NewItem (`self.BP_AttachActor`) "None" "SnapToTarget" "SnapToTarget" "SnapToTarget" true))

(fn `ChangeCanMainSound`
  (params (CanPlay :type Boolean))
  (bind _bp_soundmap (`self.BP_SoundMap`))
  (bind _audio (`/Game/Sound/BP_SoundMap.Audio` _bp_soundmap))
  (`/Engine/EditorBlueprintResources/StandardMacros.IsValid` _bp_soundmap
    (:`Is Valid`
      (`/Engine/EditorBlueprintResources/StandardMacros.IsValid` _audio
        (:`Is Valid`
          (if CanPlay
            (`ActorComponent.Activate` _audio false)
            (else
              (`ActorComponent.Deactivate` _audio))))))))

(fn `GetFromPool`
  (params (WeaponClass :type "Actor Class Reference"))
  (returns (`Is Find` :type Boolean) (WeaponInstance :type "/Game/Core/Blueprints/Weapons/BP_BaseWeapon Object Reference"))
  (locals (Weapon :type "/Game/Core/Blueprints/Weapons/BP_BaseWeapon Object Reference"))
  (for _array_element (`self.WeaponsClasses`)
    (bind _returnvalue (== (`GameplayStatics.GetObjectClass` _array_element) WeaponClass))
    (if _returnvalue
      (set `self.IsFind` _returnvalue)
      (set `local.Weapon` _array_element)))
  (`KismetArrayLibrary.Array_RemoveItem` (`self.WeaponsClasses`) (`local.Weapon`))
  (`/Engine/EditorBlueprintResources/StandardMacros.IsValid` (`local.Weapon`)
    (:`Is Valid`
      (return (`self.IsFind`) (`local.Weapon`)))
    (:`Is Not Valid`
      (return false null))))

(fn `UserConstructionScript`)