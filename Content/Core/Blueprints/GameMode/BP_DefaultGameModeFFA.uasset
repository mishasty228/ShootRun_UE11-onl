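; BP_DefaultGameModeFFA is a game mode, apparently free-for-all, that tracks when a match ends and restarts.
; At BeginPlay it binds match dispatchers and the OnDestroyed event of each existing, controlled BP_CharacterBase.
; Each such destruction counts all Controller actors, not surviving characters, and fires OnMachEnd when one or fewer remain.
; The dispatcher handlers toggle an EndMatch flag, which gates the Restart event's OnMatchReStart call, with debug prints along the way.
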(event `self.ReceiveBeginPlay`
  (`parent.ReceiveBeginPlay`)
  (add `self.OnMachEnd` (delegate `EndMatch`))
  (add `self.OnMatchReStart` (delegate `OnMatchStarted`))
  (bind _outactors (`GameplayStatics.GetAllActorsOfClass` "/Game/Core/Blueprints/Character/Base/BP_CharacterBase.BP_CharacterBase_C"))
  (for _array_element _outactors
    (`/Engine/EditorBlueprintResources/StandardMacros.IsValid` (`Pawn.GetController` _array_element)
      (:`Is Valid`
        (add `Actor.OnDestroyed` _array_element (delegate `OnDestroy`))))))

(event `OnDestroy`
  (params (DestroyedActor :type "Actor Object Reference"))
  (bind _outactors (`GameplayStatics.GetAllActorsOfClass` "/Script/Engine.Controller"))
  (`KismetSystemLibrary.PrintString` "Hello")
  (if (not (> (`KismetArrayLibrary.Array_Length` _outactors) 1))
    (`self.OnMachEnd`)))

(event `EndMatch`
  (`KismetSystemLibrary.PrintString` "end match")
  (set `self.bEndMatch` true))

(event `OnMatchStarted`
  (`KismetSystemLibrary.PrintString` "restart  match")
  (set `self.bEndMatch` false))

(event `Restart`
  (if (`self.bEndMatch`)
    (`self.OnMatchReStart`)))

(fn `UserConstructionScript`
  (`parent.UserConstructionScript`))