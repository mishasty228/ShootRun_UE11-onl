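; Test game mode that provides a timed slow-motion effect and a simple weapon pool.
; BPITimeDilation halves global time with a tick sound, ignores repeat calls while active, and restores normal time on a timer.
; AddToPool stores items and snaps them onto the level's BP_AttachActor found at BeginPlay.
; GetFromPool removes and returns an instance matching the requested class, with a found flag.
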(event `self.ReceiveBeginPlay`
  (bind _returnvalue (`GameplayStatics.GetActorOfClass` "/Game/Core/Blueprints/Weapons/BP_AttachActor.BP_AttachActor_C"))
  (set `self.BP_AttachActor` _returnvalue))

(event `/Game/Core/Blueprints/interfaces/BPI_Interact.BPI_TimeDilation`
  (params (Duration :type "Float (double-precision)"))
  (if (not (`self.IsTimeDilation`))
    (bind _returnvalue (`GameplayStatics.SpawnSound2D` "/Game/Core/Assets/Sound/Effects/SC_Tick.SC_Tick" 1.0 1.0 0.0 null))
    (set `self.DilationSoundEffect` _returnvalue)
    (`GameplayStatics.SetGlobalTimeDilation` 0.5)
    (set `self.IsTimeDilation` true)
    (bind _returnvalue_2 (`KismetSystemLibrary.K2_SetTimerDelegate` (delegate `EndTimeDilation`) Duration))
    (set `self.TimerTimeDilation` _returnvalue_2)))

(event `EndTimeDilation`
  (set `self.IsTimeDilation` false)
  (`GameplayStatics.SetGlobalTimeDilation` 1.0)
  (`AudioComponent.Stop` (`self.DilationSoundEffect`))
  (`KismetSystemLibrary.K2_ClearAndInvalidateTimerHandle` (`self.TimerTimeDilation`)))

(fn `AddToPool`
  (params (NewItem :type "/Game/Core/Blueprints/Weapons/BP_BaseWeapon Object Reference"))
  (`KismetArrayLibrary.Array_Add` (`self.WeaponsClasses`) NewItem)
  (`self.K2_AttachToActor` NewItem (`self.BP_AttachActor`) "None" "SnapToTarget" "SnapToTarget" "SnapToTarget" true))

(fn `GetFromPool`
  (params (WeaponClass :type "Object Class Reference"))
  (returns (`Is Find` :type Boolean) (WeaponInstance :type "/Game/Core/Blueprints/Weapons/BP_BaseWeapon Object Reference"))
  (locals (Weapon :type "/Game/Core/Blueprints/Weapons/BP_BaseWeapon Object Reference"))
  (for _array_element (`self.WeaponsClasses`)
    (if (== (`GameplayStatics.GetObjectClass` _array_element) WeaponClass)
      (set `local.Weapon` _array_element)))
  (bind _returnvalue (`KismetArrayLibrary.Array_RemoveItem` (`self.WeaponsClasses`) (`local.Weapon`)))
  (return _returnvalue (`local.Weapon`)))

(fn `UserConstructionScript`)