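; BP_CreateRoom is an environment actor that places a room in the level through a Child Actor component.
; On BeginPlay it sets the component's class to a random entry from Rooms when Random is on, otherwise to RoomClass.
; With ShowPreview on, the construction script applies RoomClass as a preview, without yet checking for editor mode (marked TODO).
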(event `self.ReceiveBeginPlay`
  (bind _rooms (`self.Rooms`))
  (if (`self.bRandom`)
    (`self.Create Room` (`|GetArrayItem` _rooms (`KismetMathLibrary.RandomInteger` (`KismetArrayLibrary.Array_Length` _rooms))))
    (else
      (`self.Create Room` (`self.Room Class`)))))

(fn `Create Room`
  (params (RoomClass :type "Actor Class Reference"))
  (`ChildActorComponent.SetChildActorClass` (`self.ChildActor`) RoomClass))

(fn `UserConstructionScript`
  ; TODO change to check we in editor mode
  (if (`self.bShowPreview`)
    (`self.Create Room` (`self.Room Class`))))