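; BP_Arena is an arena environment Blueprint that switches between its own audio and the game's main sound.
; Ending overlap with FirstEnterTriggerBox2 activates the arena Audio and disables main sound through the BP_DefaultGameMode cached at BeginPlay.
; Ending overlap with FirstEnterTriggerBox reverses this, but only while the CanPlaySound flag is set.
; Neither trigger filters the overlapping actor.
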(event `self.ReceiveBeginPlay`
  (bind _asbp_default_game_mode (cast `/Game/Core/Blueprints/GameMode/BP_DefaultGameMode` (`GameplayStatics.GetGameMode`)))
  (set `self.BP Default Game Mode` _asbp_default_game_mode))

(event `self.FirstEnterTriggerBox.OnComponentBeginOverlap`
  (params (OverlappedComponent :type "PrimitiveComponent Object Reference") (OtherActor :type "Actor Object Reference") (OtherComp :type "PrimitiveComponent Object Reference") (OtherBodyIndex :type Integer) (bFromSweep :type Boolean) (SweepResult :type "HitResult Structure (by ref)")))

(event `self.FirstEnterTriggerBox.OnComponentEndOverlap`
  (params (OverlappedComponent :type "PrimitiveComponent Object Reference") (OtherActor :type "Actor Object Reference") (OtherComp :type "PrimitiveComponent Object Reference") (OtherBodyIndex :type Integer))
  (if (`self.Can Play Sound`)
    (set `self.Can Play Sound` false)
    (`self.PlaySound` false)
    (`/Game/Core/Blueprints/GameMode/BP_DefaultGameMode.ChangeCanMainSound` (`self.BP Default Game Mode`) true)))

(event `self.FirstEnterTriggerBox2.OnComponentEndOverlap`
  (params (OverlappedComponent :type "PrimitiveComponent Object Reference") (OtherActor :type "Actor Object Reference") (OtherComp :type "PrimitiveComponent Object Reference") (OtherBodyIndex :type Integer))
  (set `self.Can Play Sound` true)
  (`self.PlaySound` true)
  (`/Game/Core/Blueprints/GameMode/BP_DefaultGameMode.ChangeCanMainSound` (`self.BP Default Game Mode`) false))

(fn `PlaySound`
  (params (CanPlaySound :type Boolean))
  (if CanPlaySound
    (`ActorComponent.Activate` (`self.Audio`) false)
    (else
      (`ActorComponent.Deactivate` (`self.Audio`)))))

(fn `UserConstructionScript`)