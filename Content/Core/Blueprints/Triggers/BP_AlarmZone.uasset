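; Trigger zone that switches the alarm on while the player is inside its box and off when they leave.
; Two seconds after BeginPlay it caches every BP_Wall actor in the level.
; Box overlap events filtered to BP_Player call AlarmOn or AlarmOff, which forward the same call to each cached wall.
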(event `self.ReceiveBeginPlay`
  (`KismetSystemLibrary.PrintString` "Hello")
  (`KismetSystemLibrary.Delay` 2.0)
  (bind _outactors (`GameplayStatics.GetAllActorsOfClass` "/Game/Core/Blueprints/Triggers/BP_Wall.BP_Wall_C"))
  (set `self.Walls` _outactors))

(event `self.Box.OnComponentBeginOverlap`
  (params (OverlappedComponent :type "PrimitiveComponent Object Reference") (OtherActor :type "Actor Object Reference") (OtherComp :type "PrimitiveComponent Object Reference") (OtherBodyIndex :type Integer) (bFromSweep :type Boolean) (SweepResult :type "HitResult Structure (by ref)"))
  (cast `/Game/Core/Blueprints/Player/BP_Player` OtherActor)
  (`self.AlarmOn`))

(event `self.Box.OnComponentEndOverlap`
  (params (OverlappedComponent :type "PrimitiveComponent Object Reference") (OtherActor :type "Actor Object Reference") (OtherComp :type "PrimitiveComponent Object Reference") (OtherBodyIndex :type Integer))
  (cast `/Game/Core/Blueprints/Player/BP_Player` OtherActor)
  (`self.AlarmOff`))

(fn `AlarmOff`
  (for _array_element (`self.Walls`)
    (`/Game/Core/Blueprints/Triggers/BP_Wall.AlarmOff` _array_element)))

(fn `AlarmOn`
  (for _array_element (`self.Walls`)
    (`/Game/Core/Blueprints/Triggers/BP_Wall.AlarmOn` _array_element)))

(fn `UserConstructionScript`
  (`KismetSystemLibrary.PrintString` "construct"))