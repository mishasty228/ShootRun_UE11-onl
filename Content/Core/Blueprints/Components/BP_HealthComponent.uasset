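; BP_HealthComponent is an actor component that tracks health and death for its owner.
; On BeginPlay it binds to the owner's OnTakeAnyDamage event and passes the damage to ApplyDamage.
; While alive, ApplyDamage subtracts health, fires the OnUpdateHealth dispatcher and plays a damage sound at the owner's location.
; When health reaches zero or below, it sets Dead and fires OnDead, so further damage is ignored.
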(event `self.ReceiveBeginPlay`
  (add `Actor.OnTakeAnyDamage` (`self.GetOwner`) (delegate `OnTakeAnyDamage_Event`)))

(event `OnTakeAnyDamage_Event`
  (params (DamagedActor :type "Actor Object Reference") (Damage :type "Float (single-precision)") (DamageType :type "DamageType Object Reference") (InstigatedBy :type "Controller Object Reference") (DamageCauser :type "Actor Object Reference"))
  (`self.ApplyDamage` Damage))

(fn `ApplyDamage`
  (params (Value :type "Float (double-precision)"))
  (if (not (`self.Dead`))
    (bind _output_get (set `self.Health` (- (`self.Health`) Value)))
    (`self.OnUpdateHealth`)
    (`GameplayStatics.SpawnSoundAtLocation` "/Game/Core/Assets/Sound/Damage/SCue_TakeDamage_Cue.SCue_TakeDamage_Cue" (`Actor.K2_GetActorLocation` (`self.GetOwner`)) (struct) 1.0 1.0 0.0 null null)
    (bind _returnvalue (<= _output_get 0.0))
    (if _returnvalue
      (set `self.Dead` _returnvalue)
      (`self.OnDead`))))