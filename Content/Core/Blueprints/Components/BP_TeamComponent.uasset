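; Team component that records which team its owner belongs to and whether that team counts as the enemy.
; Init stores the given TeamId and switches on it, treating 0 as friendly and 1 as enemy, with only the latter setting the Enemy flag.
; Both cases print a debug string, BeginPlay does nothing, and an older if/else version of the check remains unconnected.
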(fn `Init`
  (params (TeamId :type Integer))
  (set `self.TeamId` TeamId)
  (switch `int` (`self.TeamId`)
    (:`0`
      (`KismetSystemLibrary.PrintString` (`KismetStringLibrary.Concat_StrStr` "Team is :" (`KismetStringLibrary.Conv_IntToString` (`self.TeamId`)) "___" "I'm friendly")))
    (:`1`
      (`KismetSystemLibrary.PrintString` (`KismetStringLibrary.Concat_StrStr` "Team is :" (`KismetStringLibrary.Conv_IntToString` (`self.TeamId`)) "___" "Im' enemy"))
      (set `self.Enemy` true))))