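; BP_Player is the player character Blueprint, providing sprint and throw actions.
; SprintOn and SprintOff set the Sprint flag and swap the movement component's max walk speed, while a separate CanSprint check disallows right or backward movement.
; Throw spawns the configured ThrowClass at the player's transform with the player as owner and instigator.
; TryInteract is an empty stub, and no input wiring or callers appear here.
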(fn `CanSprint`
  (returns (ReturnValue :type Boolean))
  (return (and (not (`self.RightMove`)) (not (`self.Back`)))))

(fn `SprintOff`
  (set `self.Sprint` false)
  (set `CharacterMovementComponent.MaxWalkSpeed` (`self.Max Walk Speed`) (`self.CharacterMovement`)))

(fn `SprintOn`
  (set `self.Sprint` true)
  (set `CharacterMovementComponent.MaxWalkSpeed` (`self.SprintSpeed`) (`self.CharacterMovement`)))

(fn `Throw`
  (`|SpawnActorFromClass` (`self.ThrowClass`) (`self.GetTransform`) "Undefined" "MultiplyWithRoot" self self))

(fn `TryInteract`)

(fn `UserConstructionScript`)