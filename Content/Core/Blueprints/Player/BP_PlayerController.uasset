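; Player controller that routes Enhanced Input for moving, yaw look, sprinting, firing and weapon switching to the controlled character.
; PossesNewPawn toggles possession between the original character and a new pawn, swapping player and robot mapping contexts and remembering the previous character.
; On BeginPlay it caches the weapon component, binds to its value updates and loads the fire count.
; Save and load helpers persist that count in a device-specific SG_Statistics slot.
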(event `self.ReceiveBeginPlay`
  (bind _returnvalue (pcsubsystem `EnhancedInputLocalPlayerSubsystem` self))
  (`/Engine/EditorBlueprintResources/StandardMacros.IsValid` _returnvalue
    (:`Is Valid`
      (`EnhancedInputSubsystemInterface.AddMappingContext` _returnvalue "/Game/Core/Input/IMC_PlayerBase.IMC_PlayerBase" 0 (struct))
      (bind _asbp_player (cast `/Game/Core/Blueprints/Player/BP_Player` (`self.K2_GetPawn`)))
      (bind _output_get (set `self.BP Character` _asbp_player))
      (bind _bp_weaponcomponent (`/Game/Core/Blueprints/Character/Base/BP_CharacterBase.BP_WeaponComponent` _output_get)
        (:`then`
          (bind _output_get_2 (set `self.BP Weapon Component` _bp_weaponcomponent))
          (add `/Game/Core/Blueprints/Components/BP_WeaponComponent.UpdatedValues` _output_get_2 (`|CreateDelegate` :!event `SaveWeaponStatistics`))
          (`self.LoadWeaponStatistics`))
        (:`else`)))))

(event `EnhancedInput|/Game/Core/Input/Actions/IA_Sprint`
  (params (ActionValue :type Boolean) (ElapsedSeconds :type "Float (double-precision)") (TriggeredSeconds :type "Float (double-precision)") (InputAction :type "InputAction Object Reference" :default "/Game/Core/Input/Actions/IA_Sprint.IA_Sprint"))
  (bind _bp_character (`self.BP Character`))
  (bind _bp_character_2 (`self.BP Character`))
  ; Enchanted Input Action
  (:`Started`
    (`/Engine/EditorBlueprintResources/StandardMacros.IsValid` _bp_character_2
      (:`Is Valid`
        (`/Game/Core/Blueprints/Player/BP_Player.SprintOn` _bp_character_2))))
  (:`Completed`
    (`/Engine/EditorBlueprintResources/StandardMacros.IsValid` _bp_character
      (:`Is Valid`
        (`/Game/Core/Blueprints/Player/BP_Player.SprintOff` _bp_character)))))

(event `EnhancedInput|/Game/Core/Input/Actions/IA_Move`
  (params (ActionValue :type "Vector2D Structure") (ElapsedSeconds :type "Float (double-precision)") (TriggeredSeconds :type "Float (double-precision)") (InputAction :type "InputAction Object Reference" :default "/Game/Core/Input/Actions/IA_Move.IA_Move"))
  (bind (_returnvalue_roll _returnvalue_pitch _returnvalue_yaw) (`KismetMathLibrary.BreakRotator` (`self.GetControlRotation`)))
  (bind (_returnvalue_roll_2 _returnvalue_pitch_2 _returnvalue_yaw_2) (`KismetMathLibrary.BreakRotator` (`self.GetControlRotation`)))
  (bind _bp_character (`self.BP Character`))
  ; Enchanted Input Action
  (:`Triggered`
    (set `self.Action Value X` ActionValue_X)
    (set `self.Action Value Y` ActionValue_Y)
    (set `self.Back` (<= ActionValue_Y 0.0))
    (`/Engine/EditorBlueprintResources/StandardMacros.IsValid` _bp_character
      (:`Is Valid`
        (`Pawn.AddMovementInput` _bp_character (`KismetMathLibrary.GetForwardVector` (`KismetMathLibrary.MakeRotator` _returnvalue_roll_2 _returnvalue_pitch_2 _returnvalue_yaw_2)) (`self.Action Value Y`) false)
        (`Pawn.AddMovementInput` (`self.BP Character`) (`KismetMathLibrary.GetRightVector` (`KismetMathLibrary.MakeRotator` 0.0 _returnvalue_pitch _returnvalue_yaw)) (`self.Action Value X`) false)))))

(event `EnhancedInput|/Game/Core/Input/Actions/IA_Look`
  (params (ActionValue :type "Vector2D Structure") (ElapsedSeconds :type "Float (double-precision)") (TriggeredSeconds :type "Float (double-precision)") (InputAction :type "InputAction Object Reference" :default "/Game/Core/Input/Actions/IA_Look.IA_Look"))
  (bind _bp_character (`self.BP Character`))
  ; Enchanted Input Action
  ;; Look Up
  (:`Triggered`
    (`/Engine/EditorBlueprintResources/StandardMacros.IsValid` _bp_character
      (:`Is Valid`
        (`Pawn.AddControllerYawInput` _bp_character ActionValue_X)))))

(event `EnhancedInput|/Game/Core/Input/Actions/IA_Fire`
  (params (ActionValue :type Boolean) (ElapsedSeconds :type "Float (double-precision)") (TriggeredSeconds :type "Float (double-precision)") (InputAction :type "InputAction Object Reference" :default "/Game/Core/Input/Actions/IA_Fire.IA_Fire"))
  (bind _bp_character (`self.BP Character`))
  ; Enchanted Input Action
  (:`Triggered`
    (`/Engine/EditorBlueprintResources/StandardMacros.IsValid` _bp_character
      (:`Is Valid`
        (`/Game/Core/Blueprints/Character/Base/BP_CharacterBase.Fire` _bp_character)))))

(event `EnhancedInput|/Game/Core/Input/Actions/IA_NextWeapon`
  (params (ActionValue :type Boolean) (ElapsedSeconds :type "Float (double-precision)") (TriggeredSeconds :type "Float (double-precision)") (InputAction :type "InputAction Object Reference" :default "/Game/Core/Input/Actions/IA_NextWeapon.IA_NextWeapon"))
  ; Enchanted Input Action
  (:`Triggered`
    (`/Engine/EditorBlueprintResources/StandardMacros.IsValid` (`self.BP Character`)
      (:`Is Valid`
        (`/Game/Core/Blueprints/Character/Base/BP_CharacterBase.ChangeWeapon` (`self.BP Character`))))))

(fn `CanSprint`
  (returns (ReturnValue :type Boolean))
  (return false))

(fn `GetNewCharacter`
  (params (`BP New Pawn` :type "/Game/Core/Blueprints/Player/BP_Player Object Reference"))
  (locals (NewLocalVar :type "/Game/Core/Blueprints/ControlledPawns/BP_RobotHelper Object Reference"))
  (bind _returnvalue (pcsubsystem `EnhancedInputLocalPlayerSubsystem` self))
  (`EnhancedInputSubsystemInterface.RemoveMappingContext` (pcsubsystem `EnhancedInputLocalPlayerSubsystem` self) (`self.Mapping Context`) (struct))
  (`/Engine/EditorBlueprintResources/StandardMacros.IsValid` (`self.BP Prev Character`)
    (:`Is Valid`
      (set `self.BP Character` (`self.BP Prev Character`))
      (set `self.BP Prev Character` null)
      (set `self.Mapping Context` (`self.PlayerContext`)))
    (:`Is Not Valid`
      (set `self.BP Prev Character` (`self.BP Character`))
      (set `self.BP Character` (`local.BP New Pawn`))
      (set `self.Mapping Context` (`self.RobotContext`))))
  (`/Engine/EditorBlueprintResources/StandardMacros.IsValid` _returnvalue
    (:`Is Valid`
      (`EnhancedInputSubsystemInterface.AddMappingContext` _returnvalue (`self.Mapping Context`) 0 (struct))
      (return))))

(fn `GetWeaponStatName`
  (returns (ReturnValue :type String))
  (return (`KismetStringLibrary.Concat_StrStr` (`KismetSystemLibrary.GetDeviceId`) "WeaponStats")))

(fn `LoadWeaponStatistics`
  (bind _returnvalue (`GameplayStatics.LoadGameFromSlot` (`self.GetWeaponStatName`)))
  (bind _assg_statistics (cast `/Game/Core/Data/SG_Statistics` _returnvalue))
  (set `/Game/Core/Blueprints/Components/BP_WeaponComponent.FireCounted` (`/Game/Core/Data/SG_Statistics.FireCount` _assg_statistics) (`self.BP Weapon Component`)))

(fn `PossesNewPawn`
  (params (`BP New Pawn` :type "/Game/Core/Blueprints/Player/BP_Player Object Reference"))
  (`self.GetNewCharacter` `BP New Pawn`)
  (`self.Possess` (`self.BP Character`)))

(fn `SaveWeaponStatistics`
  (locals (SGO :type "/Game/Core/Data/SG_Statistics Object Reference"))
  (bind _sgo (`local.SGO`))
  (bind _returnvalue (`GameplayStatics.CreateSaveGameObject` "/Game/Core/Data/SG_Statistics.SG_Statistics_C"))
  (set `local.SGO` _returnvalue)
  (`/Engine/EditorBlueprintResources/StandardMacros.IsValid` _sgo
    (:`Is Valid`
      (bind _bp_weapon_component (`self.BP Weapon Component`)
        (:`then`
          (set `/Game/Core/Data/SG_Statistics.FireCount` (`/Game/Core/Blueprints/Components/BP_WeaponComponent.FireCounted` _bp_weapon_component) _sgo)
          (`GameplayStatics.SaveGameToSlot` (`local.SGO`) (`self.GetWeaponStatName`)))
        (:`else`)))))

(fn `UserConstructionScript`)