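; BP_MobBase is the base enemy character, adding AI weapon state, voice sounds and mine placement to its parent.
; It initializes its health widget, caches its AI controller on possession and updates the HasWeapon Blackboard key when a weapon is added.
; Firing and the health component's OnDead event, bound to OnCriticalHealth, play timer-throttled sounds.
; ActivateMine spawns a mine when its montage completes, then signals that activation finished.
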(event `self.ReceiveBeginPlay`
  (bind _returnvalue (`WidgetComponent.GetWidget` (`self.HealthWidget`)))
  (`parent.ReceiveBeginPlay`)
  (add `/Game/Core/Blueprints/Components/BP_HealthComponent.OnDead` (`self.BP_HealthComponent`) (delegate `OnCriticalHealth`))
  (`/Engine/EditorBlueprintResources/StandardMacros.IsValid` _returnvalue
    (:`Is Valid`
      (bind _aswbp_health (cast `/Game/Core/UI/PlayerStats/WBP_Health` _returnvalue))
      (`/Game/Core/UI/PlayerStats/WBP_Health.Init` _aswbp_health self))))

(event `OnCriticalHealth`
  (if (`self.bCanPlayCriticalSound`)
    (`GameplayStatics.SpawnSoundAttached` (`self.CriticalHealthSound`) (`self.RootComponent`) "None" (0.0 0.0 0.0) (struct) "KeepRelativeOffset" false 1.0 1.0 0.0 null null)
    (set `self.bCanPlayCriticalSound` false)
    (`KismetSystemLibrary.K2_SetTimerDelegate` (delegate `ResetCanCriticalSound`) (`self.DelayCanPlayCriticalSound`))))

(event `ResetCanCriticalSound`
  (set `self.bCanPlayCriticalSound` true))

(event `self.ReceivePossessed`
  (params (NewController :type "Controller Object Reference"))
  (bind _asbp_base_mob_ai_controller (cast `/Game/Core/Blueprints/AI/BP_BaseMobAiController` (`AIBlueprintHelperLibrary.GetAIController` NewController)))
  (set `self.BP Base Mob Ai Controller` _asbp_base_mob_ai_controller))

(event `ActivateMine`
  (`|PlayMontage` (`self.Mesh`) "/Game/Core/Blueprints/Player/Animations/AM_ActivateMine.AM_ActivateMine"
    (:`OnCompleted`
      (`|SpawnActorFromClass` (`self.MineClass`) (`KismetMathLibrary.MakeTransform` (`KismetMathLibrary.MakeVector` (.x (`self.K2_GetActorLocation`)) (.y (`self.K2_GetActorLocation`)))) "Undefined" "MultiplyWithRoot" self false null)
      (`self.OnMineActivateFinished`))))

(event `StopActivateMine`
  (`AnimInstance.Montage_Stop` (`SkeletalMeshComponent.GetAnimInstance` (`self.Mesh`)) 0.0 "/Game/Core/Blueprints/Player/Animations/AM_ActivateMine.AM_ActivateMine"))

(fn `AddWeapon`
  (params (WeaponClass :type "/Game/Core/Blueprints/Weapons/BP_BaseWeapon Class Reference"))
  (`parent.AddWeapon` WeaponClass)
  (`self.UpdateWeapon`))

(fn `Fire`
  (`parent.Fire`)
  (`self.PlayCombatSound`))

(fn `PlayCombatSound`
  (if (`self.bCanPlayCombatSound`)
    (`GameplayStatics.SpawnSoundAttached` "/Game/Assets/Sounds/Droid_Announcer/wav/03_Target_Acquired.03_Target_Acquired" (`self.RootComponent`) "None" (0.0 0.0 0.0) (struct) "KeepRelativeOffset" false 1.0 1.0 0.0 null null)
    (set `self.bCanPlayCombatSound` false)
    (`KismetSystemLibrary.K2_SetTimer` null "ResetCanPlayCombatSound" (`self.DelayCombatPlaySound`))))

(fn `ResetCanPlayCombatSound`
  (set `self.bCanPlayCombatSound` true))

(fn `UpdateWeapon`
  (bind _bp_base_mob_ai_controller (`self.BP Base Mob Ai Controller`))
  (bind _blackboard (`AIController.Blackboard` (`self.BP Base Mob Ai Controller`)))
  (`/Engine/EditorBlueprintResources/StandardMacros.IsValid` _bp_base_mob_ai_controller
    (:`Is Valid`
      (`/Engine/EditorBlueprintResources/StandardMacros.IsValid` (`AIController.Blackboard` _bp_base_mob_ai_controller)
        (:`Is Valid`
          (`/Engine/EditorBlueprintResources/StandardMacros.IsValid` (`/Game/Core/Blueprints/Components/BP_WeaponComponent.CurrentWeapon` (`self.BP_WeaponComponent`))
            (:`Is Valid`
              (`BlackboardComponent.SetValueAsBool` _blackboard (`self.HasWeapon`) true))
            (:`Is Not Valid`
              (`BlackboardComponent.SetValueAsBool` _blackboard (`self.HasWeapon`) false))))))))

(fn `UserConstructionScript`)