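; Base AI mob character with melee attacks, mine planting, a team identity and a health bar widget.
; Melee montage toggles an overlap collision that applies damage and halts movement until it completes; a mine montage spawns a mine when finished.
; Weapon changes update the AI controller's HasWeapon blackboard key.
; Team ID initializes the team component and tints a dynamic body material.
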(event `MelleAttack`
  (bind _charactermovement (`self.CharacterMovement`))
  (bind _attack_collision (`self.Attack Collision`))
  (if (not (`self.isPlayAnimAttack`))
    (`|PlayMontage` (`self.Mesh`) "/Game/Core/Blueprints/Player/Animations/Smash_Montage.Smash_Montage"
      (:`then`
        (`PrimitiveComponent.SetCollisionEnabled` _attack_collision "QueryOnly")
        (set `CharacterMovementComponent.MaxWalkSpeed` 0.0 _charactermovement)
        (set `self.isPlayAnimAttack` true))
      (:`OnCompleted`
        (`PrimitiveComponent.SetCollisionEnabled` _attack_collision "NoCollision")
        (set `CharacterMovementComponent.MaxWalkSpeed` 600.0 _charactermovement)
        (set `self.isPlayAnimAttack` false)))))

(event `self.ReceiveBeginPlay`
  (bind _returnvalue (`WidgetComponent.GetWidget` (`self.HealthBar`)))
  (`parent.ReceiveBeginPlay`)
  (`/Game/Core/Blueprints/Components/BP_TeamComponent.Init` (`self.BP_TeamComponent`) (`self.TeamId`))
  (`PrimitiveComponent.SetCollisionEnabled` (`self.Attack Collision`) "NoCollision")
  (`/Engine/EditorBlueprintResources/StandardMacros.IsValid` _returnvalue
    (:`Is Valid`
      (bind _aswbp_health (cast `/Game/Core/UI/PlayerStats/WBP_Health` _returnvalue))
      (`/Game/Core/UI/PlayerStats/WBP_Health.Init` _aswbp_health self)
      (`self.UpdateWeapon`)
      (`self.SetTeamColor`))))

(event `self.ReceivePossessed`
  (params (NewController :type "Controller Object Reference"))
  (bind _asbp_base_mob_ai_controller (cast `/Game/Core/Blueprints/AI/BP_BaseMobAiController` (`AIBlueprintHelperLibrary.GetAIController` NewController)))
  (set `self.BP Base Mob Ai Controller` _asbp_base_mob_ai_controller))

(event `self.Attack Collision.OnComponentBeginOverlap`
  (params (OverlappedComponent :type "PrimitiveComponent Object Reference") (OtherActor :type "Actor Object Reference") (OtherComp :type "PrimitiveComponent Object Reference") (OtherBodyIndex :type Integer) (bFromSweep :type Boolean) (SweepResult :type "HitResult Structure (by ref)"))
  (if (!= OtherActor self)
    (`GameplayStatics.ApplyDamage` OtherActor 10.0)))

(event `ActivateMine`
  (`|PlayMontage` (`self.Mesh`) "/Game/Core/Blueprints/Player/Animations/A_ActivateMine_Montage.A_ActivateMine_Montage"
    (:`OnCompleted`
      (`|SpawnActorFromClass` (`self.MineClass`) (`KismetMathLibrary.MakeTransform` (`KismetMathLibrary.MakeVector` (.x (`self.K2_GetActorLocation`)) (.y (`self.K2_GetActorLocation`)))) "Undefined" "MultiplyWithRoot" self false null)
      (`self.OnMineActivateFinished`))))

(event `StopActivateMine`
  (`AnimInstance.Montage_Stop` (`SkeletalMeshComponent.GetAnimInstance` (`self.Mesh`)) 0.0 null))

(fn `AddWeapon`
  (params (WeaponClass :type "/Game/Core/Blueprints/Weapons/BP_BaseWeapon Class Reference"))
  (`parent.AddWeapon` WeaponClass)
  (`self.UpdateWeapon`))

(fn `SetTeamColor`
  (bind _returnvalue (`PrimitiveComponent.CreateDynamicMaterialInstance` (`self.Mesh`) 1 "/Game/Core/Blueprints/Player/Mesh/VanguardBodyMat_Inst.VanguardBodyMat_Inst" "TeamColor"))
  (set `self.MaterialInst` _returnvalue)
  (for _array_element (`self.TeamColorStructure`)
    (if (== (break `/Game/Core/Blueprints/Data/S_TeamColor` _array_element) (`self.TeamId`))
      (`MaterialInstanceDynamic.SetVectorParameterValue` (`self.MaterialInst`) "TeamColor" (`.Color_6_16510ECD408B20C792717AB69EA24601` (break `/Game/Core/Blueprints/Data/S_TeamColor` _array_element))))))

(fn `UpdateWeapon`
  (bind _bp_base_mob_ai_controller (`self.BP Base Mob Ai Controller`))
  (bind _blackboard (`AIController.Blackboard` (`self.BP Base Mob Ai Controller`)))
  (`/Engine/EditorBlueprintResources/StandardMacros.IsValid` _bp_base_mob_ai_controller
    (:`Is Valid`
      (`/Engine/EditorBlueprintResources/StandardMacros.IsValid` (`AIController.Blackboard` _bp_base_mob_ai_controller)
        (:`Is Valid`
          (`/Engine/EditorBlueprintResources/StandardMacros.IsValid` (`/Game/Core/Blueprints/Components/BP_WeaponComponent.CurrentWeapon` (`self.BP_WeaponComponent`))
            (:`Is Valid`
              (`BlackboardComponent.SetValueAsBool` _blackboard (`self.HasWeapon`) true))
            (:`Is Not Valid`
              (`BlackboardComponent.SetValueAsBool` _blackboard (`self.HasWeapon`) false))))))))

(fn `UserConstructionScript`)