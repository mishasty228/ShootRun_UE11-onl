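; BP_CharacterBase is a base character that carries weapons and drops its current one as loot when it dies.
; Fire, ChangeWeapon and AddWeapon forward to BPWeaponComponent, while BPHealthComponent's OnDead event drives death.
; On death it spawns a BP_PickableItem with the current weapon's class, then destroys that weapon and itself.
; The pickup always receives the SKM_Lasgun mesh, whatever the weapon class.
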(event `self.ReceiveBeginPlay`
  (add `/Game/Core/Blueprints/Components/BP_HealthComponent.OnDead` (`self.BP_HealthComponent`) (delegate `OnDead`)))

(event `OnDead`
  (bind _currentweapon (`/Game/Core/Blueprints/Components/BP_WeaponComponent.CurrentWeapon` (`self.BP_WeaponComponent`)))
  (`self.SpawnLoot`)
  (`/Engine/EditorBlueprintResources/StandardMacros.IsValid` _currentweapon
    (:`Is Valid`
      (`self.K2_DestroyActor` _currentweapon))
    (:`Is Not Valid`
      _))
  (`self.K2_DestroyActor`))

(fn `AddWeapon`
  (params (WeaponClass :type "/Game/Core/Blueprints/Weapons/BP_BaseWeapon Class Reference"))
  (bind _bp_weaponcomponent (`self.BP_WeaponComponent`))
  (`/Engine/EditorBlueprintResources/StandardMacros.IsValid` _bp_weaponcomponent
    (:`Is Valid`
      (`/Game/Core/Blueprints/Components/BP_WeaponComponent.SpawnWeapon` _bp_weaponcomponent WeaponClass))))

(fn `ChangeWeapon`
  (`/Game/Core/Blueprints/Components/BP_WeaponComponent.ChangeWeapon` (`self.BP_WeaponComponent`)))

(fn `Fire`
  (`/Game/Core/Blueprints/Components/BP_WeaponComponent.Fire` (`self.BP_WeaponComponent`)))

(fn `SpawnLoot`
  (bind _currentweapon (`/Game/Core/Blueprints/Components/BP_WeaponComponent.CurrentWeapon` (`self.BP_WeaponComponent`)))
  (`/Engine/EditorBlueprintResources/StandardMacros.IsValid` _currentweapon
    (:`Is Valid`
      (`|SpawnActorFromClass` "/Game/Core/Blueprints/InteractiveObjects/BP_PickableItem.BP_PickableItem_C" (`self.GetTransform`) "Undefined" "MultiplyWithRoot" self (`GameplayStatics.GetObjectClass` _currentweapon) "/Game/Fab/SCI-FI_Rifle_Free_/scifi_rifle_2/StaticMeshes/SKM_Lasgun.SKM_Lasgun" null))))

(fn `UserConstructionScript`)