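; BP_SpawnerEnemy is an enemy spawner that places EnemyClass actors at random points inside its Box volume.
; The Spawner event starts a looping timer on DelaySpawnEnemy, but nothing in this graph triggers it, as BeginPlay is empty.
; Each tick of the timer spawns one enemy, adjusted for collision, while HowManyEnemys is below MaxCountEnemys.
; The graph never updates that count itself.
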(event `self.ReceiveBeginPlay`)

(event `Spawner`
  (`KismetSystemLibrary.K2_SetTimerDelegate` (delegate `MakeCountEnemys`) (`self.DelaySpawnEnemy`) true true))

(event `MakeCountEnemys`
  (bind _box (`self.Box`))
  (if (< (`self.HowManyEnemys`) (`self.MaxCountEnemys`))
    (`|SpawnActorFromClass` (`self.EnemyClass`) (`KismetMathLibrary.MakeTransform` (`KismetMathLibrary.RandomPointInBoundingBox` (`SceneComponent.K2_GetComponentLocation` _box) (`BoxComponent.GetScaledBoxExtent` _box))) "AdjustIfPossibleButAlwaysSpawn" "MultiplyWithRoot" null null)))

(fn `UserConstructionScript`)