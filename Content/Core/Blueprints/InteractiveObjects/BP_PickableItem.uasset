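; BP_PickableItem is a world pickup that gives the player a weapon when they walk into it.
; On BeginPlay it applies its configured skeletal mesh to the displayed component.
; When BP_Player overlaps the interaction sphere, it plays a weapon pickup sound, calls AddWeapon on the player with its weapon class, then destroys itself.
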(event `self.ReceiveBeginPlay`
  (`SkeletalMeshComponent.SetSkeletalMeshAsset` (`self.SkeletalMesh`) (`self.New Mesh`)))

(event `self.SphereInteractCollision.OnComponentBeginOverlap`
  (params (OverlappedComponent :type "PrimitiveComponent Object Reference") (OtherActor :type "Actor Object Reference") (OtherComp :type "PrimitiveComponent Object Reference") (OtherBodyIndex :type Integer) (bFromSweep :type Boolean) (SweepResult :type "HitResult Structure (by ref)"))
  (if (!= OtherActor (`self.GetOwner`))
    (bind _asbp_player (cast `/Game/Core/Blueprints/Player/BP_Player` OtherActor))
    (`GameplayStatics.SpawnSoundAtLocation` "/Game/Core/Assets/Sound/Effects/SC_WeaponPickup.SC_WeaponPickup" (`self.K2_GetActorLocation`) (struct) 1.0 1.0 0.0 null null)
    (`/Game/Core/Blueprints/Character/Base/BP_CharacterBase.AddWeapon` _asbp_player (`self.WeaponClass`))
    (`self.K2_DestroyActor`)))

(fn `UserConstructionScript`)