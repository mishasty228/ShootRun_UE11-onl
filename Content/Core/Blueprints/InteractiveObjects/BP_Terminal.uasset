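; Interactive terminal that hands player control to a robot helper in its room.
; On interact it disables further interaction, then searches the child actors of BPRoom for a BP_RobotHelper and stores the reference.
; It then has BP_PlayerController possess that robot as the new pawn.
; CanInteract is exposed through the interaction interface and is never re-enabled in this Blueprint.
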(event `/Game/Core/Blueprints/Interfaces/BPI_Interact.BPI_Interact`
  (bind _bp_room (`self.BP_Room`))
  (set `self.Can Interact` false)
  (`/Engine/EditorBlueprintResources/StandardMacros.IsValid` _bp_room
    (:`Is Valid`
      (for _array_element (`self.GetAllChildActors` _bp_room true)
        (bind _asbp_robot_helper (cast `/Game/Core/Blueprints/ControlledPawns/BP_RobotHelper` _array_element))
        (set `self.As BP Robot Helper` _asbp_robot_helper))
      (`KismetSystemLibrary.PrintString` "interact ")
      (bind _asbp_player_controller (cast `/Game/Core/Blueprints/Player/BP_PlayerController` (`GameplayStatics.GetPlayerController` 0)))
      (`/Game/Core/Blueprints/Player/BP_PlayerController.PossesNewPawn` _asbp_player_controller (`self.As BP Robot Helper`)))))

(fn `BPI_CanIneract`
  (returns (bCanInteract :type Boolean))
  (return (`self.Can Interact`)))

(fn `UserConstructionScript`)