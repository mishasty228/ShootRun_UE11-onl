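; BP_Button is a test interactable button that destroys the actors in its related-objects array when used.
; It binds to an interact delegate on BeginPlay and also implements an interact interface event, so both routes call DestroyRelatedObjects.
; DestroyRelatedObjects destroys each valid entry in the array, and only the delegate route prints a debug string first.
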(event `self.ReceiveBeginPlay`
  (add `self.EventInteractDelegate` (delegate `OnInteractDelegate`)))

(event `OnInteractDelegate`
  (`KismetSystemLibrary.PrintString` "OnInteractDelegate")
  (`self.DestroyRelatedObjects`))

(event `/Game/Core/Blueprints/Interfaces/BPI_Interact.BPI_Interact`
  (`self.DestroyRelatedObjects`))

(fn `DestroyRelatedObjects`
  (for _array_element (`self.ArrRelatedObjects`)
    (`/Engine/EditorBlueprintResources/StandardMacros.IsValid` _array_element
      (:`Is Valid`
        (`self.K2_DestroyActor` _array_element)))))

(fn `UserConstructionScript`)