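; Base projectile actor for weapons that damages what it hits, using ammo data for damage, initial speed and an optional custom mesh.
; On spawn it ignores itself and sets a fixed velocity, first in local space, then overwritten by a raw X-axis vector.
; Box overlap applies damage and destroys the projectile unless the other actor is on the ignore list and not exactly of the base projectile class.
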(event `self.ReceiveBeginPlay`
  (`self.Init`))

(event `self.Box.OnComponentBeginOverlap`
  (params (OverlappedComponent :type "PrimitiveComponent Object Reference") (OtherActor :type "Actor Object Reference") (OtherComp :type "PrimitiveComponent Object Reference") (OtherBodyIndex :type Integer) (bFromSweep :type Boolean) (SweepResult :type "HitResult Structure (by ref)"))
  (bind _ammodata_danage (break `/Game/Core/Blueprints/Data/S_AmmoData` (`self.AmmoData`)))
  (if (not (and (`KismetArrayLibrary.Array_Contains` (`self.IgnoreActors`) OtherActor) (!= (`GameplayStatics.GetObjectClass` OtherActor) "BP_ProjectileBase_C")))
    (`GameplayStatics.ApplyDamage` OtherActor _ammodata_danage)
    (`self.K2_DestroyActor`)))

(fn `Init`
  (bind _projectilemovement (`self.ProjectileMovement`))
  (bind (_ammodata_danage _ammodata_initialspeed _ammodata_busecustommesh _ammodata_custommesh) (break `/Game/Core/Blueprints/Data/S_AmmoData` (`self.AmmoData`)))
  (`KismetArrayLibrary.Array_Add` (`self.IgnoreActors`) self)
  (set `ProjectileMovementComponent.InitialSpeed` _ammodata_initialspeed _projectilemovement)
  (`ProjectileMovementComponent.SetVelocityInLocalSpace` _projectilemovement (7000.0 0.0 0.0))
  (set `MovementComponent.Velocity` (7000.0 0.0 0.0) (`self.ProjectileMovement`))
  (if (and _ammodata_busecustommesh (`KismetSystemLibrary.IsValid` _ammodata_custommesh))
    (`StaticMeshComponent.SetStaticMesh` (`self.StaticMesh`) _ammodata_custommesh)))

(fn `UserConstructionScript`)