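; BP_Molotov is a Molotov actor that spawns a damage area when it hits something.
; Its Capsule's begin-overlap event ignores the owner and other Molotovs, then disables the capsule's collision.
; It spawns a BP_DamageBox using only the actor's X and Y location, leaving height unset, and destroys itself.
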(event `self.Capsule.OnComponentBeginOverlap`
  (params (OverlappedComponent :type "PrimitiveComponent Object Reference") (OtherActor :type "Actor Object Reference") (OtherComp :type "PrimitiveComponent Object Reference") (OtherBodyIndex :type Integer) (bFromSweep :type Boolean) (SweepResult :type "HitResult Structure (by ref)"))
  (bind (_returnvalue_x _returnvalue_y) (`KismetMathLibrary.BreakVector` (`self.K2_GetActorLocation`)))
  (if (and (!= OtherActor (`self.GetOwner`)) (!= (`GameplayStatics.GetObjectClass` OtherActor) "BP_Molotov_C"))
    (`PrimitiveComponent.SetCollisionEnabled` (`self.Capsule`) "NoCollision")
    (`|SpawnActorFromClass` "/Game/Core/Blueprints/Weapons/Molotov/BP_DamageBox.BP_DamageBox_C" (`KismetMathLibrary.MakeTransform` (`KismetMathLibrary.MakeVector` _returnvalue_x _returnvalue_y)) "Undefined" "MultiplyWithRoot" null null)
    (`/Engine/EditorBlueprintResources/StandardMacros.IsValid` self
      (:`Is Valid`
        (`self.K2_DestroyActor`)))))

(fn `UserConstructionScript`)