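; BP_Rifle is a child weapon Blueprint that fires a projectile from its muzzle with a rifle sound.
; Fire is gated by CanFire, which it clears before calling the parent Fire, SpawnProjectile and the sound.
; SpawnProjectile reads the ammo's data table row and spawns AmmoClass at the Muzzle socket, passing that row and ignoring the owner and rifle.
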(event `self.Fire`
  (if (`self.CanFire`)
    (set `self.CanFire` false)
    (`parent.Fire`)
    (`self.SpawnProjectile`)
    (`GameplayStatics.SpawnSoundAtLocation` "/Game/Core/Assets/Sound/Fire/SCue_FireRifle.SCue_FireRifle" (`self.K2_GetActorLocation`) (struct) 1.0 1.0 0.0 null null)))

(fn `SpawnProjectile`
  (bind (_ammorow_datatable _ammorow_rowname) (break `DataTableRowHandle` (`self.AmmoRow`)))
  (bind _ammoclass (`self.AmmoClass`)
    (:`then`
      (bind _returnvalue (`|GetDataTableRow` _ammorow_datatable _ammorow_rowname)
        (:`then`
          (`|SpawnActorFromClass` _ammoclass (`SceneComponent.GetSocketTransform` (`self.SkeletalMesh`) "Muzzle" "RTS_World") "Undefined" "MultiplyWithRoot" null _returnvalue (`|MakeArray` (`self.GetOwner`) self :!type "Actor Object Reference") null))))
    (:`else`)))

(fn `UserConstructionScript`
  (`parent.UserConstructionScript`))