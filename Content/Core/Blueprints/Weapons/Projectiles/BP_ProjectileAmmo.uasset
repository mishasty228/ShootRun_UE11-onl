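; Projectile actor for weapon ammo, taking its speed, damage, impact effect and optional custom mesh from AmmoData.
; On BeginPlay it ignores itself and listed actors, then launches along local X.
; Box overlaps with non-ignored actors apply damage through the owner's instigator controller and explode; stopping also explodes.
; Explosion async-loads the soft-referenced impact system, spawns it, and destroys the projectile only if that reference is valid.
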(event `self.ReceiveBeginPlay`
  (`self.Init`))

(event `self.Box.OnComponentBeginOverlap`
  (params (OverlappedComponent :type "PrimitiveComponent Object Reference") (OtherActor :type "Actor Object Reference") (OtherComp :type "PrimitiveComponent Object Reference") (OtherBodyIndex :type Integer) (bFromSweep :type Boolean) (SweepResult :type "HitResult Structure (by ref)"))
  (bind _returnvalue (`self.GetOwner`))
  (bind (_ammodata_speed _ammodata_damage) (break `/Game/Core/Blueprints/Weapons/Projectiles/FAmmoData` (`self.AmmoData`)))
  (bind _returnvalue_2 (`self.GetInstigatorController` _returnvalue))
  (if (not (`KismetArrayLibrary.Array_Contains` (`self.ActorsToIgnore`) OtherActor))
    (`/Engine/EditorBlueprintResources/StandardMacros.IsValid` _returnvalue
      (:`Is Valid`
        (`/Engine/EditorBlueprintResources/StandardMacros.IsValid` _returnvalue_2
          (:`Is Valid`
            (`GameplayStatics.ApplyDamage` OtherActor _ammodata_damage _returnvalue_2 _returnvalue "/Script/Engine.DamageType")
            (`self.Explosion`)))))))

(event `self.ProjectileMovement.OnProjectileStop`
  (params (ImpactResult :type "HitResult Structure (by ref)"))
  (`KismetSystemLibrary.PrintString` "Stop")
  (`self.Explosion`))

(event `self.ProjectileMovement.OnComponentDeactivated`
  (params (Component :type "ActorComponent Object Reference"))
  (`KismetSystemLibrary.PrintString` "Deactivate"))

(event `Explosion`
  (bind (_ammodata_speed _ammodata_damage _ammodata_busecustommesh _ammodata_custommesh _ammodata_impactsystem) (break `/Game/Core/Blueprints/Weapons/Projectiles/FAmmoData` (`self.AmmoData`)))
  (`|LoadAsset` _ammodata_impactsystem
    (:`Completed`
      (if (`KismetSystemLibrary.IsValidSoftObjectReference` _ammodata_impactsystem)
        (bind _returnvalue (`NiagaraFunctionLibrary.SpawnSystemAtLocation` (`|ConvertAsset` _ammodata_impactsystem) (`self.K2_GetActorLocation`)))
        (`/Engine/EditorBlueprintResources/StandardMacros.IsValid` _returnvalue
          (:`Is Valid`
            (`SceneComponent.K2_DetachFromComponent` _returnvalue "KeepWorld" "KeepWorld" "KeepWorld" true))
          (:`Is Not Valid`
            _))
        (`self.K2_DestroyActor`)))))

(fn `Init`
  (bind _projectilemovement (`self.ProjectileMovement`))
  (bind (_ammodata_speed _ammodata_damage _ammodata_busecustommesh _ammodata_custommesh) (break `/Game/Core/Blueprints/Weapons/Projectiles/FAmmoData` (`self.AmmoData`)))
  (bind _actorstoignore (`self.ActorsToIgnore`))
  (`KismetArrayLibrary.Array_Add` _actorstoignore self)
  (for _array_element _actorstoignore
    (`PrimitiveComponent.IgnoreActorWhenMoving` (`self.Box`) _array_element true)
    (`PrimitiveComponent.IgnoreActorWhenMoving` (`self.StaticMesh`) _array_element true))
  (`ProjectileMovementComponent.SetVelocityInLocalSpace` _projectilemovement (`KismetMathLibrary.MakeVector` _ammodata_speed))
  (`ActorComponent.SetActive` _projectilemovement true true)
  (if (and _ammodata_busecustommesh (`KismetSystemLibrary.IsValidSoftObjectReference` _ammodata_custommesh))
    (`StaticMeshComponent.SetStaticMesh` (`self.StaticMesh`) (`|ConvertAsset` _ammodata_custommesh))))

(fn `UserConstructionScript`)