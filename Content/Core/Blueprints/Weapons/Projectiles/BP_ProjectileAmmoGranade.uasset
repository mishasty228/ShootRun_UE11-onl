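; Grenade ammo projectile that damages the actor it hits and then explodes.
; On Box overlap it skips actors in ActorsToIgnore and requires a valid owner with an instigator controller.
; It applies the AmmoData damage with its DamageType, credited to that controller with the owner as causer, then calls Explosion, whose logic is not defined in these graphs.
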(event `self.Box.OnComponentBeginOverlap`
  (params (OverlappedComponent :type "PrimitiveComponent Object Reference") (OtherActor :type "Actor Object Reference") (OtherComp :type "PrimitiveComponent Object Reference") (OtherBodyIndex :type Integer) (bFromSweep :type Boolean) (SweepResult :type "HitResult Structure (by ref)"))
  (bind _returnvalue (`self.GetOwner`))
  (bind (_ammodata_speed _ammodata_damage) (break `/Game/Core/Blueprints/Weapons/Projectiles/FAmmoData` (`self.AmmoData`)))
  (bind _returnvalue_2 (`self.GetInstigatorController` _returnvalue))
  (if (not (`KismetArrayLibrary.Array_Contains` (`self.ActorsToIgnore`) OtherActor))
    (`/Engine/EditorBlueprintResources/StandardMacros.IsValid` _returnvalue
      (:`Is Valid`
        (`/Engine/EditorBlueprintResources/StandardMacros.IsValid` _returnvalue_2
          (:`Is Valid`
            (`GameplayStatics.ApplyDamage` OtherActor _ammodata_damage _returnvalue_2 _returnvalue "/Script/Engine.DamageType")
            (`self.Explosion`)))))))

(fn `UserConstructionScript`
  (`parent.UserConstructionScript`))