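; Projectile weapon Blueprint that extends its parent weapon's Fire event to spawn an ammo actor from the muzzle.
; SpawnProjectile looks up the ammo data table row and passes it to the spawned AmmoClass actor, ignoring the owner and weapon.
; Spawn location comes from the Muzzle socket, but direction follows the owner's forward vector rather than the socket's rotation.
; Each shot also draws a red debug arrow along that direction.
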(event `self.Fire`
  (`parent.Fire`)
  (`self.SpawnProjectile`))

(fn `SpawnProjectile`
  (bind _returnvalue (`self.GetOwner`))
  (bind (_ammorow_datatable _ammorow_rowname) (break `DataTableRowHandle` (`self.AmmoRow`)))
  (bind _returnvalue_2 (`self.GetActorForwardVector` (`self.GetOwner`)))
  (bind _location (.location (`SceneComponent.GetSocketTransform` (`self.SkeletalMesh`) "Muzzle" "RTS_World")))
  (bind _ammoclass (`self.AmmoClass`)
    (:`then`
      (bind _returnvalue_3 (`|GetDataTableRow` _ammorow_datatable _ammorow_rowname)
        (:`then`
          (`|SpawnActorFromClass` _ammoclass (`KismetMathLibrary.MakeTransform` _location (`KismetMathLibrary.Conv_VectorToRotator` _returnvalue_2) (.scale (`SceneComponent.GetSocketTransform` (`self.SkeletalMesh`) "Muzzle" "RTS_World"))) "Undefined" "MultiplyWithRoot" _returnvalue _returnvalue_3 (`|MakeArray` _returnvalue self :!type "Actor Object Reference") null)
          (`KismetSystemLibrary.DrawDebugArrow` _location (+ _location (* _returnvalue_2 200.0)) 10.0 (struct :`R` 1.0 :`A` 1.0) 5.0 5.0))))
    (:`else`)))

(fn `UserConstructionScript`
  (`parent.UserConstructionScript`))