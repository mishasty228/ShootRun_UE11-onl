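; Base weapon for characters that fires a hitscan laser, with BaseDamage doubled at BeginPlay whenever player controller 0 exists, regardless of owner.
; Fire starts a cooldown timer that re-enables CanFire and plays a random shot montage on the owning character's mesh.
; HitScanDamage, not called in this graph, traces from the muzzle, plays sound and a Niagara beam, then applies damage and reports it to AI perception.
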(event `self.ReceiveBeginPlay`
  (bind _returnvalue (`GameplayStatics.GetPlayerController` 0))
  (bind _ascharacter (cast `Character` (`self.GetOwner`)))
  (bind _output_get (set `self.Character` _ascharacter))
  (set `self.Mesh` (`Character.Mesh` _output_get))
  ; More damage for player
  (`/Engine/EditorBlueprintResources/StandardMacros.IsValid` _returnvalue
    (:`Is Valid`
      (set `self.PlayerController` _returnvalue)
      (set `self.Base Damage` (* (`self.Base Damage`) 2.0)))))

(event `Fire`
  (`self.CooldownFireEvent`)
  (`self.PlayeFireAnimation`))

(event `PlayeFireAnimation`
  (bind _arrshotanimations (`self.ArrShotAnimations`))
  (`/Engine/EditorBlueprintResources/StandardMacros.IsValid` (`self.Mesh`)
    (:`Is Valid`
      (`|PlayMontage` (`self.Mesh`) (`|GetArrayItem` _arrshotanimations (`KismetMathLibrary.RandomIntegerInRange` 0 (- (`KismetArrayLibrary.Array_Length` _arrshotanimations) 1)))))))

(event `CooldownFireEvent`
  (bind _returnvalue (`KismetSystemLibrary.K2_SetTimerDelegate` (delegate `CanFireEvent`) (`self.WeaponCooldown`)))
  (set `self.HandleFire` _returnvalue))

(event `CanFireEvent`
  (set `self.CanFire` true))

(fn `HitScanDamage`
  (bind _returnvalue (`self.GetOwner`))
  (bind _skeletalmesh (`self.SkeletalMesh`))
  (bind _startvector (`self.StartVector`))
  (bind _hit_actor (`self.Hit Actor`))
  (bind _returnvalue_2 (+ _startvector (`self.EndVector`)))
  (set `self.StartVector` (`SceneComponent.GetSocketLocation` _skeletalmesh "Muzzle"))
  (set `self.EndVector` (* (`KismetMathLibrary.GetForwardVector` (`SceneComponent.GetSocketRotation` _skeletalmesh "Muzzle")) 1000))
  (set `self.HitVector` _returnvalue_2)
  (bind _outhit (`KismetSystemLibrary.LineTraceSingle` _startvector _returnvalue_2 "TraceTypeQuery1" false (`|MakeArray` (`self.GetOwner`))))
  (`GameplayStatics.SpawnSoundAtLocation` (`self.FireSound`) (`self.StartVector`) (struct) 1.0 1.0 0.0 null null)
  (bind (_bblockinghit _binitialoverlap _time _distance _location _impactpoint _normal _impactnormal _physmat _hitactor) (`GameplayStatics.BreakHitResult` _outhit))
  (set `self.Hit Actor` _hitactor)
  (`self.PlayFireNiagara` (`KismetMathLibrary.SelectVector` _impactpoint (`self.HitVector`) _bblockinghit) "/Game/VFX/Trace/Rifle/NS_Laserbeam.NS_Laserbeam")
  (if _bblockinghit
    (`/Engine/EditorBlueprintResources/StandardMacros.IsValid` _hit_actor
      (:`Is Valid`
        (`GameplayStatics.ApplyDamage` _hit_actor (`self.Base Damage`) (`self.GetInstigatorController` _returnvalue) _returnvalue)
        (`AISense_Damage.ReportDamageEvent` (`self.Hit Actor`) (`self.Character`) 0.0 (`self.K2_GetActorLocation` (`self.Character`)))))))

(fn `PlayFireNiagara`
  (params (InValue :type "Vector Structure") (NiagaraEffect :type "NiagaraSystem Object Reference"))
  (bind _returnvalue (`NiagaraFunctionLibrary.SpawnSystemAtLocation` NiagaraEffect (`SceneComponent.GetSocketLocation` (`self.SkeletalMesh`) "Muzzle")))
  (`NiagaraComponent.SetVariableVec3` _returnvalue "TraceTarget" InValue))

(fn `ResetFire`
  (set `self.CanFire` true))

(fn `UserConstructionScript`)