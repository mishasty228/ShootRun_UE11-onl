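; BP_Flamethrower is a flamethrower weapon that damages actors in front of its muzzle.
; Fire, gated by CanFire, clears that flag, plays the fire animation and runs a wide, short multi-sphere trace along the muzzle socket's forward vector, with debug drawing on.
; Valid blocking hits receive BaseDamage, credited to the owner.
; PlayFireNiagara spawns a given Niagara effect attached to the muzzle; nothing here calls it or resets CanFire.
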(event `self.Fire`
  (bind _returnvalue (`self.GetOwner`))
  (bind _skeletalmesh (`self.SkeletalMesh`))
  (bind _startvector (`self.StartVector`))
  (bind _hit_actor (`self.Hit Actor`))
  (if (`self.CanFire`)
    (set `self.CanFire` false)
    (set `self.StartVector` (`SceneComponent.GetSocketLocation` _skeletalmesh "Muzzle"))
    (set `self.EndVector` (* (`KismetMathLibrary.GetForwardVector` (`SceneComponent.GetSocketRotation` _skeletalmesh "Muzzle")) 500))
    (`self.PlayeFireAnimation`)
    (bind _outhits (`KismetSystemLibrary.SphereTraceMulti` _startvector (+ _startvector (`self.EndVector`)) 300.0 "TraceTypeQuery1" false (`|MakeArray` (`self.GetOwner`)) "ForDuration"))
    (for _array_element _outhits
      (bind (_bblockinghit _binitialoverlap _time _distance _location _impactpoint _normal _impactnormal _physmat _hitactor) (`GameplayStatics.BreakHitResult` _array_element))
      (set `self.Hit Actor` _hitactor)
      (if _bblockinghit
        (`/Engine/EditorBlueprintResources/StandardMacros.IsValid` _hit_actor
          (:`Is Valid`
            (`GameplayStatics.ApplyDamage` _hit_actor (`self.Base Damage`) (`self.GetInstigatorController` _returnvalue) _returnvalue)))))))

(fn `PlayFireNiagara`
  (params (InValue :type "Vector Structure") (NiagaraEffect :type "NiagaraSystem Object Reference"))
  (bind _skeletalmesh (`self.SkeletalMesh`))
  (bind (_returnvalue_roll _returnvalue_pitch _returnvalue_yaw) (`KismetMathLibrary.BreakRotator` (`SceneComponent.K2_GetComponentRotation` _skeletalmesh)))
  (`NiagaraFunctionLibrary.SpawnSystemAttached` NiagaraEffect (`self.SkeletalMesh`) "Muzzle" (`SceneComponent.GetSocketLocation` _skeletalmesh "Muzzle") (`KismetMathLibrary.MakeRotator` 0.0 0.0 (- _returnvalue_yaw 90.0)) "KeepWorldPosition"))

(fn `UserConstructionScript`
  (`parent.UserConstructionScript`))